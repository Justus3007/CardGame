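; CardPlayerCamera is a player camera Blueprint that records left and right mouse button held states as booleans.
; The left button sets LMBDown directly on press and release.
; The right button sets RMBDown through two DoOnce gates that re-arm each other, so press and release alternate.
; A similar DoOnce chain for LMBDown is left disconnected, and nothing in this Blueprint reads either flag.
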(event Input|MouseEvents|RightMouseButton
  (params (Key :type Key%20Structure))
  (:Pressed
    (Utilities|FlowControl|DoOnce false :!label _label
      (:Completed
        (Variables|Default|SetRMBDown true)
        (goto _label_2 Reset))))
  (:Released
    (Utilities|FlowControl|DoOnce true :!label _label_2
      (:Completed
        (Variables|Default|SetRMBDown false)
        (goto _label Reset)))))

(event Input|MouseEvents|LeftMouseButton
  (params (Key :type Key%20Structure))
  (:Pressed
    (Variables|Default|SetLMBDown true))
  (:Released
    (Variables|Default|SetLMBDown false)))

(fn ConstructionScript)