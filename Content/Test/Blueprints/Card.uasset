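; Card actor that the player can drag around with the mouse, with physics switched off while held.
; Each tick it attaches if its Cube is hovered and the CardPlayerCamera pawn reports left mouse down, then follows a cursor line trace, hovering slightly above the hit.
; Construction gives Cube a dynamic Gladiator material, passing CardHero to a vector parameter named None.
; Hover and attach states print to screen every tick.
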(event OnBeginCursorOver(Cube)
  (params (TouchedComponent :type Primitive%20Component%20Object%20Reference))
  (Variables|Default|SetCursorHover true))

(event OnEndCursorOver(Cube)
  (params (TouchedComponent :type Primitive%20Component%20Object%20Reference))
  (Variables|Default|SetCursorHover false))

(event Custom|CheckAttach
  (if (and (Variables|Default|GetCursorHover) (Variables|/Game/Test/Blueprints/CardPlayerCamera.CardPlayerCamera_C|GetLMBDown (Variables|Default|GetPlayer)))
    (CallFunction|SetAttached true)
    (else
      (CallFunction|SetAttached false))))

(event Custom|Pick%20Up%20Mesh
  (bind _returnvalue (Game|GetPlayerController 0))
  (bind (_worldlocation _worlddirection) (Game|Player|ConvertMouseLocationToWorldSpace _returnvalue))
  (if (Variables|Default|GetAttachedToCursor)
    (bind (_outhit _returnvalue_2) (Collision|LineTraceByChannel _worldlocation (+ _worldlocation (* _worlddirection (Variables|Default|GetCursorTraceDistance))) "TraceTypeQuery3" false 0 "None"))
    (if _returnvalue_2
      (Transformation|SetActorLocation (+ (.Location (Collision|BreakHitResult _outhit)) "0, 0,30.000000") true false))))

(event MouseInput|EventActorEndCursorOver)

(event EventTick
  (params (DeltaSeconds :type Float%20%28single-precision%29))
  (CallFunction|CheckAttach)
  (CallFunction|PickUpMesh)
  (Development|PrintString (Utilities|String|ToString(Boolean) (Variables|Default|GetCursorHover)) true true "(R=1.000000,G=0.049777,B=0.000000,A=1.000000)")
  (Development|PrintString (Utilities|String|ToString(Boolean) (Variables|Default|GetAttachedToCursor))))

(event EventBeginPlay
  ;[1 1 1] Get player Reference
  (bind _ascard_player_camera (Utilities|Casting|CastToCardPlayerCamera (Pawn|GetControlledPawn (Game|GetPlayerController 0))))
  (Variables|Default|SetPlayer _ascard_player_camera))

(event MouseInput|EventActorBeginCursorOver)

(fn ConstructionScript
  (bind _cube (Variables|Default|GetCube))
  (bind _returnvalue (Rendering|Material|CreateDynamicMaterialInstance _cube 0 "/Game/Test/Blueprints/Materials/Gladiator.Gladiator" :!class /Script/Engine.PrimitiveComponent))
  (Rendering|Material|SetVectorParameterValue _returnvalue "None" (Variables|Default|GetCardHero) :!class /Script/Engine.MaterialInstanceDynamic)
  (Rendering|Material|SetMaterial _cube 0 _returnvalue))

(fn SetAttached
  (params (Attached :type Boolean))
  (Physics|SetSimulatePhysics (Variables|Default|GetStaticMesh) (not Attached))
  (Variables|Default|SetAttachedToCursor Attached))