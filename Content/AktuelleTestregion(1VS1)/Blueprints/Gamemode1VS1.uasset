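; Game mode for a local 1VS1 card match that runs the pre-game setup of player names and decks.
; BeginPlay shows the name-entry widget with UI-only input, then events swap it for deck selection and, once ready, the loading screen.
; It stores both players' names and chosen cards for retrieval, updates card counters on the deck widget, and signals it when both selections are in.
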(event Custom|SetzeName
  (params (Spieler1 :type String) (Spieler2 :type String))
  (Variables|Default|SetName1 Spieler1)
  (Variables|Default|SetName2 Spieler2))

(event Custom|Spieler1KarteHinzufügenAnzeige
  (bind _deckref (Variables|Default|GetDeckRef))
  (Default|AnzahlSetzen _deckref (Utilities|String|ToString(Integer) (+ (Math|Conversions|ToInteger(Byte) (Variables|/Game/Game/UI/Game/1VS1/Deckwählen.Deckwählen_C|GetAnzahl1 _deckref)) 1)) (Variables|/Game/Game/UI/Game/1VS1/Deckwählen.Deckwählen_C|GetAnzahl2 _deckref)))

(event Custom|Spieler2KarteHinzufügenAnzeige
  (bind _deckref (Variables|Default|GetDeckRef))
  (Default|AnzahlSetzen _deckref (Variables|/Game/Game/UI/Game/1VS1/Deckwählen.Deckwählen_C|GetAnzahl1 _deckref) (Utilities|String|ToString(Integer) (+ (Math|Conversions|ToInteger(Byte) (Variables|/Game/Game/UI/Game/1VS1/Deckwählen.Deckwählen_C|GetAnzahl2 _deckref)) 1))))

(event Custom|DeckSetzErstellen
  (Widget|RemovefromParent (Variables|Default|GetNameSetzenWBPRef))
  (bind _returnvalue (UserInterface|CreateWidget "/Game/Game/UI/Game/1VS1/Deckwählen.Deckwählen_C" (Game|GetPlayerController 0)))
  (bind _output_get (Variables|Default|SetDeckRef _returnvalue))
  (UserInterface|Viewport|AddtoViewport _output_get 0))

(event Custom|SpielStarten
  (if (Variables|Default|GetBereit)
    (Widget|RemovefromParent (Variables|Default|GetDeckRef))
    (bind _returnvalue (UserInterface|CreateWidget "/Game/Game/UI/Game/1VS1/1VS1LoadingScreen.1VS1LoadingScreen_C" (Game|GetPlayerController 0)))
    (bind _output_get (Variables|Default|Set1VS1LoadingScreenRef _returnvalue))
    (UserInterface|Viewport|AddtoViewport _output_get 0)))

(event Custom|SetzeGewählteKarten2
  (params (Spieler%202 :type Array%20of%20Integers))
  (Variables|Default|SetSpieler2Karten Spieler%202)
  (Variables|Default|SetSpieler2Bereit true)
  (CallFunction|AlleBereit))

(event Custom|SetzeGewählteKarten
  (params (Spieler1 :type Array%20of%20Integers))
  (Variables|Default|SetSpieler1Karten Spieler1)
  (Variables|Default|SetSpieler1Bereit true)
  (CallFunction|AlleBereit))

(event EventBeginPlay
  (bind _returnvalue (Game|GetPlayerController 0))
  (bind _returnvalue_2 (UserInterface|CreateWidget "/Game/Game/UI/Game/1VS1/1VS1NameSetzen.1VS1NameSetzen_C" _returnvalue))
  (bind _output_get (Variables|Default|SetNameSetzenWBPRef _returnvalue_2))
  (UserInterface|Viewport|AddtoViewport _output_get 0)
  (Input|SetInputModeUIOnly _returnvalue 0 "DoNotLock")
  (Variables|/Script/Engine.PlayerController|SetbShowMouseCursor _returnvalue true))

(event EventTick
  (params (DeltaSeconds :type Float%20%28single-precision%29)))

(fn ConstructionScript)

(fn GibNamen
  (return (Variables|Default|GetName1) (Variables|Default|GetName2)))

(fn GibKarten
  (return (Variables|Default|GetSpieler1Karten) (Variables|Default|GetSpieler2Karten)))

(fn AlleBereit
  (if (and (Variables|Default|GetSpieler1Bereit) (Variables|Default|GetSpieler2Bereit))
    (Default|Bereit (Variables|Default|GetDeckRef))
    (Variables|Default|SetBereit true)
    (else
      (Variables|Default|SetBereit false)))
  (return (Variables|Default|GetBereit)))